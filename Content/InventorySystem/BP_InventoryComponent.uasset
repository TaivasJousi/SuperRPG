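; Inventory component that stores item stacks in a slot array and toggles a centered inventory window on the SuperRPG player controller's HUD.
; PrepareInventory sizes the array and refreshes item data from class defaults on BeginPlay and before the window opens.
; AddToInventory fills partial stacks or claims empty slots, with AddToStack feeding overflow back into it recursively.
; InventoryQuery checks whether a class's total quantity meets a requested amount.
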(event EventBeginPlay
  (CallFunction|PrepareInventory))

(fn ToggleInventory
  (bind _returnvalue (Game|GetPlayerController 0))
  (bind _returnvalue_2 (Game|GetPlayerController 0))
  ;[1 1 1] Check if widget exists
  (Variables|Default|GetInventoryWindow
    (:then
      ;[1 1 1] Widget exists - remove it, adjust controls
      (Widget|RemovefromParent (Variables|Default|GetInventoryWindow))
      (Variables|Default|SetInventoryWindow 0)
      (Input|SetInputModeGameOnly _returnvalue)
      (Variables|/Script/Engine.PlayerController|SetbShowMouseCursor _returnvalue false))
    (:else
      ;[1 1 1] Create Inventory Window Widget
      (CallFunction|PrepareInventory)
      (bind _returnvalue_3 (UserInterface|CreateWidget "/Game/InventorySystem/InventoryUI/InventoryWindow.InventoryWindow_C" 0 self))
      (Variables|Default|SetInventoryWindow _returnvalue_3)
      (bind _asbp_player_controller_super_rpg (Utilities|Casting|CastToBP_PlayerController_SuperRPG (Game|GetPlayerController 0)))
      (bind _returnvalue_4 (Class|CanvasPanel|AddChildtoCanvas (Variables|/Game/InventorySystem/InventoryUI/HUD.HUD_C|GetHUD_Canvas (Variables|/Game/Blueprints/Framework/BP_PlayerController_SuperRPG.BP_PlayerController_SuperRPG_C|GetHUDWidget _asbp_player_controller_super_rpg)) (Variables|Default|GetInventoryWindow)))
      ;[1 1 1] Set size | Set alignment to center | Set anchors to center | Set position
      (Class|CanvasPanelSlot|SetAutoSize _returnvalue_4 true)
      (Class|CanvasPanelSlot|SetAlignment _returnvalue_4 "(X=0.500000,Y=0.500000)")
      (Class|CanvasPanelSlot|SetAnchors _returnvalue_4 (Utilities|Struct|MakeAnchors "(X=0.500000,Y=0.500000)" "(X=0.500000,Y=0.500000)"))
      (Class|CanvasPanelSlot|SetPosition _returnvalue_4 (Variables|Default|GetPosition))
      ;[1 1 1] Use mouse in widget
      (Input|SetInputModeUIOnly _returnvalue_2 (Variables|Default|GetInventoryWindow) "LockAlways")
      (Variables|/Script/Engine.PlayerController|SetbShowMouseCursor _returnvalue_2 true))))

(fn PrepareInventory
  ;[1 1 1] Resize array
  (Utilities|Array|Resize (Variables|Default|GetInventory) (Variables|Default|GetNumberOfSlots))
  ;[1 1 1] Check whether or not class set
  (for (_array_element _array_index) (Variables|Default|GetInventory)
    ;[1 1 1] If no class found set new one
    (if (!= (.Class (Utilities|Struct|BreakS_ItemStructure (.itemstructure _array_element))) 0)
      (Utilities|Array|SetArrayElem (Variables|Default|GetInventory) _array_index (Utilities|Struct|MakeS_SlotStructure (Utilities|GetClassDefaults (.Class (Utilities|Struct|BreakS_ItemStructure (.itemstructure _array_element)))) (.quantity _array_element))))))

(fn CreateStack
  (params (ContentToAdd :type S%20Slot%20Structure%20Structure))
  ;[1 1 1] Check for space
  (bind (_array_element _array_index) (Utilities|Array|ForEachLoopwithBreak (Variables|Default|GetInventory) :!label _label)
    (:LoopBody
      (if (<= (.quantity _array_element) 0)
        (LocalVariables|SetHasSpace true)
        (LocalVariables|SetIdentifiedIndex _array_index)
        (goto _label Break)))
    (:Completed
      ;[1 1 1] Check the loop result: whether the variable is set
      (if (LocalVariables|GetHasSpace)
        ;[1 1 1] Variable set - meaning it has gone through loop - meaning there is space - create new stack
        (Utilities|Array|SetArrayElem (Variables|Default|GetInventory) (LocalVariables|GetIdentifiedIndex) ContentToAdd)
        (return (LocalVariables|GetHasSpace))
        (else
          ;[1 1 1] No space
          (return false))))))

(fn AddtoStack
  (params (SlotStructure :type S%20Slot%20Structure%20Structure) (SlotIndex :type Integer))
  (bind _inventory (Variables|Default|GetInventory))
  (bind _inventory_2 (Variables|Default|GetInventory))
  (bind _maxstacksize (Utilities|Struct|BreakS_ItemStructure (.itemstructure SlotStructure)))
  (bind _output (Utilities|Array|Get(acopy) _inventory_2 SlotIndex))
  (bind _output_2 (Utilities|Array|Get(acopy) _inventory SlotIndex))
  ;[1 1 1] Check how many items in partial stack already - to local variable
  (bind _output_get (LocalVariables|SetCurrentQuantity (.quantity _output_2)))
  ;[1 1 1] If new amount exceeds max stack size - fill existing and create new stack
  (if (> (+ _output_get (.Quantity (Utilities|Struct|BreakS_SlotStructure SlotStructure))) (.MaxStackSize (Utilities|Struct|BreakS_ItemStructure (.itemstructure _output_2))))
    ;[1 1 1] Fill existing stack till max
    (Utilities|Array|SetArrayElem (Variables|Default|GetInventory) SlotIndex (Utilities|Struct|MakeS_SlotStructure (.itemstructure SlotStructure) _maxstacksize))
    ;[1 1 1] Add remaining to stack
    (CallFunction|AddtoInventory (Utilities|Struct|MakeS_SlotStructure (.itemstructure SlotStructure) (- (.quantity SlotStructure) (- _maxstacksize (LocalVariables|GetCurrentQuantity)))))
    (else
      ;[1 1 1] Add item to partial stack: same item, new quantity
      (Utilities|Array|SetArrayElem _inventory_2 SlotIndex (Utilities|Struct|MakeS_SlotStructure (.itemstructure _output) (+ (.quantity _output) (.quantity SlotStructure))))))
  (return true))

(fn InventoryQuery
  (params (QueryItem :type BP%20Item%20Class%20Reference) (QueryAmount :type Integer))
  ;[1 1 1] Check for item and amount of it; return whether or not running total equal to query amount
  (bind _array_element (Utilities|Array|ForEachLoopwithBreak (Variables|Default|GetInventory))
    (:LoopBody
      (if (== (.Class (Utilities|Struct|BreakS_ItemStructure (.itemstructure _array_element))) QueryItem)
        (LocalVariables|SetRunningTotal (+ (.quantity _array_element) (LocalVariables|GetRunningTotal)))))
    (:Completed
      (return (>= (LocalVariables|GetRunningTotal) QueryAmount)))))

(fn AddtoInventory
  (params (ContentToAdd :type S%20Slot%20Structure%20Structure))
  ;[1 1 1] Check for stackable: if is - check for existing stack, if not - create new. Check for partial stack: if exists - add to it, if not - create new stack.
  (if (.IsStackable (Utilities|Struct|BreakS_ItemStructure (.itemstructure ContentToAdd)))
    (bind _stackindex (Utilities|HasPartialStack ContentToAdd)
      (:True
        (bind _success (CallFunction|AddtoStack ContentToAdd _stackindex))
        (LocalVariables|SetIsSuccessful _success))
      (:False
        (bind _success_2 (CallFunction|CreateStack ContentToAdd :!label _label))
        (LocalVariables|SetIsSuccessful _success_2)))
    (else
      (goto _label)))
  (return (LocalVariables|GetIsSuccessful)))