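; BP_Item is an inventory item actor that can be picked up through Interact, with a UseItem function that returns false.
; Interact adds one unit to the interactor's BP_InventoryComponent; on success it destroys the actor and shows a notification through the main hero's health bar widget.
; Box overlaps toggle the mesh's custom depth and stencil for an outline, checking player character 0's class rather than the overlapping actor.
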(event OnComponentBeginOverlap(BoxCollision)
  (params (OverlappedComponent :type Primitive%20Component%20Object%20Reference) (OtherActor :type Actor%20Object%20Reference) (OtherComp :type Primitive%20Component%20Object%20Reference) (OtherBodyIndex :type Integer) (bFromSweep :type Boolean) (SweepResult :type Hit%20Result%20Structure%20%28by%20ref%29))
  (bind _staticmesh (Variables|Default|GetStaticMesh))
  ;[1 1 1] Outline material active when box collision overlaped
  (Utilities|Casting|CastToBP_MainHero (Game|GetPlayerCharacter 0))
  (Rendering|SetRenderCustomDepth _staticmesh true)
  (Rendering|SetCustomDepthStencilValue _staticmesh 2))

(event OnComponentEndOverlap(BoxCollision)
  (params (OverlappedComponent :type Primitive%20Component%20Object%20Reference) (OtherActor :type Actor%20Object%20Reference) (OtherComp :type Primitive%20Component%20Object%20Reference) (OtherBodyIndex :type Integer))
  (bind _staticmesh (Variables|Default|GetStaticMesh))
  ;[1 1 1] Outline material active when box collision overlaped
  (Utilities|Casting|CastToBP_MainHero (Game|GetPlayerCharacter 0))
  (Rendering|SetRenderCustomDepth _staticmesh false)
  (Rendering|SetCustomDepthStencilValue _staticmesh 0))

(event EventInteract
  (params (Interactor :type Actor%20Object%20Reference))
  ;[1 1 1] Adding to inventory and calling the notification
  (bind _success (Default|AddtoInventory (Actor|GetComponentbyClass Interactor "/Game/InventorySystem/BP_InventoryComponent.BP_InventoryComponent_C") (Utilities|Struct|MakeS_SlotStructure (Variables|Default|GetItemStructure) 1)))
  (if _success
    (Actor|DestroyActor)
    (bind _asbp_main_hero (Utilities|Casting|CastToBP_MainHero (Game|GetPlayerCharacter 0)))
    (Default|ShowNotificationBox (Variables|/Game/Blueprints/Characters/BP_MainHero.BP_MainHero_C|GetWB_HealthBar _asbp_main_hero))))

(fn ConstructionScript)

(fn UseItem
  (return false))