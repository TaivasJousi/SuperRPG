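; BP_Item_Bush is an inventory item, a herb that restores a small amount of the player's health when used.
; It overrides UseItem, calls the parent, then casts the player character to BP_MainHero to add to HitPoints, clamped to the valid range.
; It then pushes the new value directly to the hero's health bar widget and reports success.
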(fn ConstructionScript
  (|CallParentFunction))

(fn UseItem
  ;[1 1 1] Usage of herb: access to player's health - add points to health - clamp between 0 and 100 - set new health - update health bar
  (|CallParentFunction)
  (bind _asbp_main_hero (Utilities|Casting|CastToBP_MainHero (Game|GetPlayerCharacter 0)))
  (bind _output_get (Variables|/Script/SuperRPG.BaseCharacter|SetHitPoints _asbp_main_hero (Math|Float|Clamp(Float) (+ (Variables|/Script/SuperRPG.BaseCharacter|GetHitPoints _asbp_main_hero) 1e+01) 0.0 1e+02)))
  (Default|UpdateHealthbar (Variables|/Game/Blueprints/Characters/BP_MainHero.BP_MainHero_C|GetWB_HealthBar _asbp_main_hero) _output_get)
  (return true))