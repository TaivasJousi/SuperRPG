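; Inventory item Blueprint that turns on the player's minimap when used.
; UseItem runs the parent logic, then creates a UI_Minimap widget and adds it to the viewport.
; It hides the hero's mesh from the Minimap component and sets the hero's Minimapexists flag.
; After a validity check, it shows the small image on the hero's existing MinimapWidget, not the new widget, and returns true.
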(event EventBeginPlay)

(event Collision|EventActorBeginOverlap
  (params (OtherActor :type Actor%20Object%20Reference)))

(event EventTick
  (params (DeltaSeconds :type Float%20%28single-precision%29)))

(fn ConstructionScript
  (|CallParentFunction))

(fn UseItem
  ;[1 1 1] On click set minimap widget visible
  (|CallParentFunction)
  (bind _asbp_main_hero (Utilities|Casting|CastToBP_MainHero (Game|GetPlayerCharacter 0)))
  ;[1 1 1] Minimap
  (bind _returnvalue (UserInterface|CreateWidget "/Game/Blueprints/Components/Minimap/UI_Minimap.UI_Minimap_C"))
  (UserInterface|Viewport|AddtoViewport _returnvalue 0)
  (Variables|Default|SetMinimap%20Widget (Variables|/Game/Blueprints/Characters/BP_MainHero.BP_MainHero_C|GetMinimapWidget _asbp_main_hero))
  (Class|SceneCaptureComponent|HideComponent (Variables|/Game/Blueprints/Characters/BP_MainHero.BP_MainHero_C|GetMinimap _asbp_main_hero) (Variables|/Script/Engine.Character|GetMesh _asbp_main_hero))
  (Variables|/Game/Blueprints/Characters/BP_MainHero.BP_MainHero_C|Setminimapexists _asbp_main_hero true)
  (Utilities|IsValid 0
    (:Is%20Valid
      (Widget|SetVisibility (Variables|/Game/Blueprints/Components/Minimap/UI_Minimap.UI_Minimap_C|GetMinimapSmallImage (Variables|/Game/Blueprints/Characters/BP_MainHero.BP_MainHero_C|GetMinimapWidget _asbp_main_hero)) "Visible")
      (return true))))