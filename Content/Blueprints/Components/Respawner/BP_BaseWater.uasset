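; BP_BaseWater is a water volume that records a respawn point and is meant to let the hero dive.
; Box overlap saves the hero's transform as SpawnNearWater and opens a Gate, which closes on end overlap.
; Pressing L through the open gate disables movement, plays the dive montage, waits its length, then sets Swimming mode.
; The author's note marks this work-in-progress, reporting that the gate doesn't open.
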(event OnComponentBeginOverlap(BoxCollision)
  (params (OverlappedComponent :type Primitive%20Component%20Object%20Reference) (OtherActor :type Actor%20Object%20Reference) (OtherComp :type Primitive%20Component%20Object%20Reference) (OtherBodyIndex :type Integer) (bFromSweep :type Boolean) (SweepResult :type Hit%20Result%20Structure%20%28by%20ref%29))
  ;[1 0.3785 0.3785] Not working shitcode, gate doesn't open | Idea: when overlap collision - open gate, when end overlap - close gate; in gate change movement from jump/run to dive (TODO: check collision size) | Should work: set respawn point
  (bind _asbp_main_hero (Utilities|Casting|CastToBP_MainHero OtherActor))
  (Variables|/Game/Blueprints/Characters/BP_MainHero.BP_MainHero_C|SetSpawnNearWater _asbp_main_hero (Transformation|GetActorTransform _asbp_main_hero))
  (Development|PrintString "collision")
  (Utilities|FlowControl|Gate false) ; enters at Open
)

(event OnComponentEndOverlap(BoxCollision)
  (params (OverlappedComponent :type Primitive%20Component%20Object%20Reference) (OtherActor :type Actor%20Object%20Reference) (OtherComp :type Primitive%20Component%20Object%20Reference) (OtherBodyIndex :type Integer))
  ;[1 0.3785 0.3785] Not working shitcode, gate doesn't open | Idea: when overlap collision - open gate, when end overlap - close gate; in gate change movement from jump/run to dive (TODO: check collision size) | Should work: set respawn point
  (Utilities|Casting|CastToBP_MainHero OtherActor)
  (Utilities|FlowControl|Gate false) ; enters at Close
)

(event Input|ActionEvents|InputActionJump
  (params (Key :type Key%20Structure))
  ;[1 0.3785 0.3785] Not working shitcode, gate doesn't open | Idea: when overlap collision - open gate, when end overlap - close gate; in gate change movement from jump/run to dive (TODO: check collision size) | Should work: set respawn point
)

(event Input|KeyboardEvents|L
  (params (Key :type Key%20Structure))
  ;[1 0.3785 0.3785] Not working shitcode, gate doesn't open | Idea: when overlap collision - open gate, when end overlap - close gate; in gate change movement from jump/run to dive (TODO: check collision size) | Should work: set respawn point
  (:Pressed
    (Utilities|FlowControl|Gate false
      (:Exit
        (Development|PrintString "gate open")
        (bind _asbp_main_hero (Utilities|Casting|CastToBP_MainHero (Game|GetPlayerCharacter 0)))
        (Pawn|Components|CharacterMovement|DisableMovement (Variables|/Script/Engine.Character|GetCharacterMovement _asbp_main_hero))
        (bind _returnvalue (Animation|PlayAnimMontage _asbp_main_hero "/Game/Animation/Characters/MainHero/AM_Hero_Dive.AM_Hero_Dive" 1.0 "None"))
        (Utilities|FlowControl|Delay _returnvalue)
        (Pawn|Components|CharacterMovement|SetMovementMode (Variables|/Script/Engine.Character|GetCharacterMovement _asbp_main_hero) "MOVE_Swimming" 0)))))

(fn ConstructionScript)