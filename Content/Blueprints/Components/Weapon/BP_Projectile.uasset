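; Projectile actor that targets the hero for homing, damages it on contact and expires after a few seconds.
; BeginPlay sets its lifespan and points ProjectileMovement's homing target at the capsule of the first BP_MainHero found.
; Sphere overlap with the hero subtracts ProjectileDamage directly from HitPoints, calls OnTakeDamage, then destroys the projectile.
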(event OnComponentBeginOverlap(SphereCollision)
  (params (OverlappedComponent :type Primitive%20Component%20Object%20Reference) (OtherActor :type Actor%20Object%20Reference) (OtherComp :type Primitive%20Component%20Object%20Reference) (OtherBodyIndex :type Integer) (bFromSweep :type Boolean) (SweepResult :type Hit%20Result%20Structure%20%28by%20ref%29))
  ;[1 1 1] Apply damage to hero
  (bind _asbp_main_hero (Utilities|Casting|CastToBP_MainHero OtherActor))
  (Variables|/Script/SuperRPG.BaseCharacter|SetHitPoints _asbp_main_hero (- (Variables|/Script/SuperRPG.BaseCharacter|GetHitPoints _asbp_main_hero) (Variables|Default|GetProjectileDamage)))
  (Class|BaseCharacter|OnTakeDamage _asbp_main_hero (- (Variables|/Script/SuperRPG.BaseCharacter|GetHitPoints _asbp_main_hero) (Variables|Default|GetProjectileDamage)))
  (Actor|DestroyActor))

(event Collision|EventActorBeginOverlap
  (params (OtherActor :type Actor%20Object%20Reference)))

(event EventTick
  (params (DeltaSeconds :type Float%20%28single-precision%29)))

(event EventBeginPlay
  ;[1 1 1] Destroy in 3 sec | Set homing
  (Utilities|FlowControl|Sequence
    (:then_0
      (Actor|SetLifeSpan 3.0))
    (:then_1
      (bind _outactors (Actor|GetAllActorsOfClass "/Game/Blueprints/Characters/BP_MainHero.BP_MainHero_C"))
      (Variables|/Script/Engine.ProjectileMovementComponent|SetHomingTargetComponent (Variables|Default|GetProjectileMovement) (Variables|/Script/Engine.Character|GetCapsuleComponent (Utilities|Array|Get(acopy) _outactors))))))

(fn ConstructionScript)