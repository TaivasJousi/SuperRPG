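; BP_Healer is a health pickup that heals the main hero when touched.
; On overlap with its sphere collision, it casts to BP_MainHero and adds HealPoints to HitPoints, with no clamp in this graph.
; It then shows a hardcoded "30 points healed" notice through the hero's health bar widget, refreshes the bar and destroys itself.
; The message text is independent of the HealPoints value.
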(event OnComponentBeginOverlap(SphereCollision)
  (params (OverlappedComponent :type Primitive%20Component%20Object%20Reference) (OtherActor :type Actor%20Object%20Reference) (OtherComp :type Primitive%20Component%20Object%20Reference) (OtherBodyIndex :type Integer) (bFromSweep :type Boolean) (SweepResult :type Hit%20Result%20Structure%20%28by%20ref%29))
  ;[1 1 1] Healer Collecting
  (bind _asbp_main_hero (Utilities|Casting|CastToBP_MainHero OtherActor))
  (bind _output_get (Variables|/Script/SuperRPG.BaseCharacter|SetHitPoints _asbp_main_hero (+ (Variables|/Script/SuperRPG.BaseCharacter|GetHitPoints _asbp_main_hero) (Variables|Default|GetHealPoints))))
  (bind _output_get_2 (Variables|/Game/Blueprints/Framework/WB_GeneralNotification.WB_GeneralNotification_C|SetNotificateText (Variables|/Game/Blueprints/Characters/BP_MainHero.BP_MainHero_C|GetGenNotificationWidget _asbp_main_hero) (Utilities|Text|MakeLiteralText "30 points healed")))
  (Default|ShowGeneralNotBox (Variables|/Game/Blueprints/Characters/BP_MainHero.BP_MainHero_C|GetWB_HealthBar _asbp_main_hero) _output_get_2)
  (Default|UpdateHealthbar (Variables|/Game/Blueprints/Characters/BP_MainHero.BP_MainHero_C|GetWB_HealthBar _asbp_main_hero) _output_get)
  (Actor|DestroyActor))

(event EventBeginPlay)

(event Collision|EventActorBeginOverlap
  (params (OtherActor :type Actor%20Object%20Reference)))

(event EventTick
  (params (DeltaSeconds :type Float%20%28single-precision%29)))

(fn ConstructionScript)