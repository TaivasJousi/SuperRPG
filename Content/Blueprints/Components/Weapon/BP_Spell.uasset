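; BP_Spell is a collectible spell pickup that adds to the main hero's spell count on overlap.
; Its collision sphere casts the overlapping actor to BP_MainHero, increases SpellCount, then shows a notification and refreshes the count through the health bar widget.
; It then toggles mesh and particle visibility and disables collision, reversing both after a cooldown delay so the pickup becomes collectible again.
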(event OnComponentBeginOverlap(SphereCollectCollision)
  (params (OverlappedComponent :type Primitive%20Component%20Object%20Reference) (OtherActor :type Actor%20Object%20Reference) (OtherComp :type Primitive%20Component%20Object%20Reference) (OtherBodyIndex :type Integer) (bFromSweep :type Boolean) (SweepResult :type Hit%20Result%20Structure%20%28by%20ref%29))
  ;[1 1 1] Spell Collecting
  (bind _asbp_main_hero (Utilities|Casting|CastToBP_MainHero OtherActor))
  (Variables|/Game/Blueprints/Characters/BP_MainHero.BP_MainHero_C|SetSpellCount _asbp_main_hero (+ (Variables|/Game/Blueprints/Characters/BP_MainHero.BP_MainHero_C|GetSpellCount _asbp_main_hero) (Variables|Default|GetAddedSpell)))
  (bind _output_get (Variables|/Game/Blueprints/Framework/WB_GeneralNotification.WB_GeneralNotification_C|SetNotificateText (Variables|/Game/Blueprints/Characters/BP_MainHero.BP_MainHero_C|GetGenNotificationWidget _asbp_main_hero) (Utilities|Text|MakeLiteralText "Spell collected")))
  (Default|ShowGeneralNotBox (Variables|/Game/Blueprints/Characters/BP_MainHero.BP_MainHero_C|GetWB_HealthBar _asbp_main_hero) _output_get)
  (Default|UpdateSpellCount (Variables|/Game/Blueprints/Characters/BP_MainHero.BP_MainHero_C|GetWB_HealthBar _asbp_main_hero))
  (Development|PrintString "Spell collected!")
  (Rendering|ToggleVisibility (Variables|Default|GetSpellMesh) false)
  (Collision|SetCollisionEnabled (Variables|Default|GetSphereCollectCollision) "NoCollision")
  (Utilities|FlowControl|Delay (Variables|Default|GetCoolDownTime))
  (Rendering|ToggleVisibility (Variables|Default|GetSpellMesh) false)
  (Collision|SetCollisionEnabled (Variables|Default|GetSphereCollectCollision) "QueryAndPhysics"))

(fn ConstructionScript)