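; BP_Shield is a shield pickup that gives BP_MainHero a full shield.
; Sphere overlap refills ShieldDefence1 to 100, sets the hero's HaveShield, shows and updates the health bar's shield widget, then destroys the actor.
; Box overlap subtracts temporary damage only when the player-character cast fails; its comment flags it as probably broken.
; Both overlaps check player character 0 rather than the overlapping actor.
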(event OnComponentBeginOverlap(SphereSphere)
  (params (OverlappedComponent :type Primitive%20Component%20Object%20Reference) (OtherActor :type Actor%20Object%20Reference) (OtherComp :type Primitive%20Component%20Object%20Reference) (OtherBodyIndex :type Integer) (bFromSweep :type Boolean) (SweepResult :type Hit%20Result%20Structure%20%28by%20ref%29))
  ;[1 1 1] Shield Collecting
  (bind _asbp_main_hero (Utilities|Casting|CastToBP_MainHero (Game|GetPlayerCharacter 0)))
  (bind _output_get (Variables|Default|SetShieldDefence1 (+ (Variables|Default|GetShieldDefence1) (- 1e+02 (Variables|Default|GetShieldDefence1)))))
  (Default|UpdateShieldBar (Variables|/Game/Blueprints/Characters/BP_MainHero.BP_MainHero_C|GetWB_HealthBar _asbp_main_hero) _output_get)
  (Variables|/Game/Blueprints/Characters/BP_MainHero.BP_MainHero_C|SetHaveShield _asbp_main_hero true)
  (Widget|SetVisibility (Variables|/Game/Blueprints/Framework/WB_Healthbar.WB_Healthbar_C|GetShieldWidget (Variables|/Game/Blueprints/Characters/BP_MainHero.BP_MainHero_C|GetWB_HealthBar _asbp_main_hero)) "Visible")
  (Actor|DestroyActor)
  (Development|PrintString "Shield collected!")
  ;;[1 0.4271 0.4271] Removing Widget | Not Checked
  (if (== (Variables|Default|GetShieldDefence1) 0.0)
    (Widget|RemovefromParent (Variables|/Game/Blueprints/Framework/WB_Healthbar.WB_Healthbar_C|GetShieldWidget (Variables|/Game/Blueprints/Characters/BP_MainHero.BP_MainHero_C|GetWB_HealthBar _asbp_main_hero)))))

(event OnComponentBeginOverlap(BoxCollision)
  (params (OverlappedComponent :type Primitive%20Component%20Object%20Reference) (OtherActor :type Actor%20Object%20Reference) (OtherComp :type Primitive%20Component%20Object%20Reference) (OtherBodyIndex :type Integer) (bFromSweep :type Boolean) (SweepResult :type Hit%20Result%20Structure%20%28by%20ref%29))
  ;[1 0.4722 0.4722] Shield Damage | Not Checked | Probably Not Working
  (Utilities|Casting|CastToBP_MainHero (Game|GetPlayerCharacter 0)
    (:CastFailed
      (Variables|Default|SetShieldDefence1 (- (Variables|Default|GetShieldDefence1) (Variables|Default|GetTemroraryDamage1)))
      (Development|PrintString "Shield damage"))))

(fn ConstructionScript)