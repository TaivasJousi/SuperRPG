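; BP_ShieldSphere is a shield that absorbs projectiles and reports its defence to the main hero's health bar.
; Activate and deactivate events toggle the particle effect and sphere collision together.
; Overlapping BP_Projectile actors subtract their shield damage from the defence, update the shield bar and are destroyed.
; At zero defence it clears the hero's HaveShield flag and hides the shield widget, without deactivating the sphere itself.
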(event OnComponentBeginOverlap(SphereCollision)
  (params (OverlappedComponent :type Primitive%20Component%20Object%20Reference) (OtherActor :type Actor%20Object%20Reference) (OtherComp :type Primitive%20Component%20Object%20Reference) (OtherBodyIndex :type Integer) (bFromSweep :type Boolean) (SweepResult :type Hit%20Result%20Structure%20%28by%20ref%29))
  ;[1 1 1] Shield damage registration in widget | Attacking projectile (spell also possible) destruction | Widget invisible when no defence left
  (bind _asbp_projectile (Utilities|Casting|CastToBP_Projectile OtherActor))
  (bind _output_get (Variables|Default|SetShieldSphereDefence (- (Variables|Default|GetShieldSphereDefence) (Variables|/Game/Blueprints/Components/Weapon/BP_Projectile.BP_Projectile_C|GetProjectileShieldDamage _asbp_projectile))))
  (bind _asbp_main_hero (Utilities|Casting|CastToBP_MainHero (Game|GetPlayerCharacter 0)))
  (Default|UpdateShieldBar (Variables|/Game/Blueprints/Characters/BP_MainHero.BP_MainHero_C|GetWB_HealthBar _asbp_main_hero) _output_get)
  (Actor|DestroyActor _asbp_projectile)
  (if (<= (Math|Float|Clamp(Float) (Variables|Default|GetShieldSphereDefence) 0.0 1e+02) 0.0)
    (Variables|/Game/Blueprints/Characters/BP_MainHero.BP_MainHero_C|SetHaveShield _asbp_main_hero false)
    (Widget|SetVisibility (Variables|/Game/Blueprints/Framework/WB_Healthbar.WB_Healthbar_C|GetShieldWidget (Variables|/Game/Blueprints/Characters/BP_MainHero.BP_MainHero_C|GetWB_HealthBar _asbp_main_hero)) "Hidden")))

(event Custom|ActivateSphereEffect
  ;[1 1 1] Activate and Deactivate particle effect and protecting collision
  (Components|Activation|SetActive (Variables|Default|GetParticleSystem) true false)
  (Collision|SetCollisionEnabled (Variables|Default|GetSphereCollision) "QueryAndPhysics"))

(event Custom|DeactivateSphereEffect
  ;[1 1 1] Activate and Deactivate particle effect and protecting collision
  (Components|Activation|SetActive (Variables|Default|GetParticleSystem) false false)
  (Collision|SetCollisionEnabled (Variables|Default|GetSphereCollision) "NoCollision"))

(event EventBeginPlay
  ;[1 1 1] Initialization
  (bind _asbp_main_hero (Utilities|Casting|CastToBP_MainHero (Game|GetPlayerCharacter 0)))
  (Variables|/Game/Blueprints/Framework/WB_Healthbar.WB_Healthbar_C|SetShieldRef (Variables|/Game/Blueprints/Characters/BP_MainHero.BP_MainHero_C|GetWB_HealthBar _asbp_main_hero) self))

(fn ConstructionScript)