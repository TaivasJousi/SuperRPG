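; Base weapon component that damages actors its mesh overlaps.
; On BeginPlay it takes its first child component as the weapon's static mesh, printing an error if the cast fails.
; It makes that mesh query-only on a custom collision object type, binds its begin-overlap event and sets it to ignore the owner when moving.
; Each overlap applies fixed damage with the owner as causer and prints a debug message.
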(event Custom|Initialize
  (params (Mesh :type Static%20Mesh%20Component%20Object%20Reference))
  (bind _asstatic_mesh_component (Utilities|Casting|CastToStaticMeshComponent (Components|GetChildComponent self 0))
    (:then
      (bind _output_get (Variables|Default|SetMainMesh _asstatic_mesh_component))
      (Collision|SetCollisionEnabled _output_get "QueryOnly")
      (Collision|SetCollisionObjectType (Variables|Default|GetMainMesh) "ECC_GameTraceChannel1")
      (Collision|AssignOnComponentBeginOverlap (Variables|Default|GetMainMesh) (delegate Custom|OnComponentBeginOverlap_Event_0)))
    (:CastFailed
      (Development|PrintString "Weapon is not static mesh component" true true "(R=0.545139,G=0.041503,B=0.026500,A=1.000000)"))))

(event Custom|OnComponentBeginOverlap_Event_0
  (params (OverlappedComponent :type Primitive%20Component%20Object%20Reference) (OtherActor :type Actor%20Object%20Reference) (OtherComp :type Primitive%20Component%20Object%20Reference) (OtherBodyIndex :type Integer) (bFromSweep :type Boolean) (SweepResult :type Hit%20Result%20Structure%20%28by%20ref%29))
  (Game|Damage|ApplyDamage OtherActor 1e+01 0 (Components|GetOwner))
  (Development|PrintString "Damage"))

(event EventBeginPlay
  (CallFunction|Initialize)
  (Collision|IgnoreActorwhenMoving (Variables|Default|GetMainMesh) (Components|GetOwner) true))

(event EventTick
  (params (DeltaSeconds :type Float%20%28single-precision%29)))