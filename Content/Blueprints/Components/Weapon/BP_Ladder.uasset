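; BP_Ladder is a climbable ladder actor that puts the player's BP_MainHero into a ladder state.
; Its box collision switches Tick on, which traces forward from the hero each frame with debug drawing and prints.
; A hit on the ladder sets OnLadder, aligns the hero's yaw to the Arrow and plays MoveToLadder, whose update logic is absent.
; Leaving the box stops Tick, clears OnLadder and restores walking mode and speed.
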(event OnComponentBeginOverlap(BoxCollision)
  (params (OverlappedComponent :type Primitive%20Component%20Object%20Reference) (OtherActor :type Actor%20Object%20Reference) (OtherComp :type Primitive%20Component%20Object%20Reference) (OtherBodyIndex :type Integer) (bFromSweep :type Boolean) (SweepResult :type Hit%20Result%20Structure%20%28by%20ref%29))
  (Actor|Tick|SetActorTickEnabled true))

(event OnComponentEndOverlap(BoxCollision)
  (params (OverlappedComponent :type Primitive%20Component%20Object%20Reference) (OtherActor :type Actor%20Object%20Reference) (OtherComp :type Primitive%20Component%20Object%20Reference) (OtherBodyIndex :type Integer))
  (bind _asbp_main_hero (Utilities|Casting|CastToBP_MainHero OtherActor))
  (Actor|Tick|SetActorTickEnabled false)
  (Variables|/Game/Blueprints/Characters/BP_MainHero.BP_MainHero_C|SetOnLadder? _asbp_main_hero false)
  (Pawn|Components|CharacterMovement|SetMovementMode (Variables|/Script/Engine.Character|GetCharacterMovement _asbp_main_hero) "MOVE_Walking" 0)
  (Variables|/Script/Engine.CharacterMovementComponent|SetMaxWalkSpeed (Variables|/Script/Engine.Character|GetCharacterMovement _asbp_main_hero) (Variables|/Game/Blueprints/Characters/BP_MainHero.BP_MainHero_C|GetMaxWalkSpeed _asbp_main_hero)))

(event EventBeginPlay
  (Actor|Tick|SetActorTickEnabled false))

(event EventTick
  (params (DeltaSeconds :type Float%20%28single-precision%29))
  (bind _asbp_main_hero (Utilities|Casting|CastToBP_MainHero (Game|GetPlayerCharacter 0)))
  (bind (_outhit _returnvalue) (Collision|LineTraceByChannel (Transformation|GetActorLocation _asbp_main_hero) (+ (Transformation|GetActorLocation _asbp_main_hero) (* (Transformation|GetActorForwardVector _asbp_main_hero) 2e+02)) "TraceTypeQuery1" false 0 "ForDuration" false))
  (Development|PrintString (Utilities|String|ToString(Boolean) _returnvalue))
  (if (== (.HitActor (Collision|BreakHitResult _outhit)) self)
    (Variables|/Game/Blueprints/Characters/BP_MainHero.BP_MainHero_C|SetOnLadder? _asbp_main_hero true)
    (Development|PrintString "on ladder")
    (Transformation|SetActorRotation _asbp_main_hero (Math|Rotator|MakeRotator (.roll (Transformation|GetActorRotation _asbp_main_hero)) (.pitch (Transformation|GetActorRotation _asbp_main_hero)) (.Yaw (Math|Rotator|BreakRotator (Transformation|GetWorldRotation (Variables|Default|GetArrow))))))
    ;[1 1 1] get actor location, arrow world location - set actor location
    (Timeline|MoveToLadder Play)))

(event Collision|EventActorBeginOverlap
  (params (OtherActor :type Actor%20Object%20Reference))
  (Utilities|Casting|CastToBP_MainHero OtherActor))

(fn ConstructionScript)