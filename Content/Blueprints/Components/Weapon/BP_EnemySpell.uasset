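; Enemy spell actor that damages the main hero or the hero's shield on contact.
; Sphere overlap casts to BP_MainHero to subtract SpellDamage from HitPoints, otherwise to BP_Shield_Child to subtract it from ShieldDefence.
; The hero branch also prints a debug value, which subtracts damage again from the updated HitPoints.
; A short lifespan set on BeginPlay removes the actor; hits do not destroy it.
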(event OnComponentBeginOverlap(SphereCollision)
  (params (OverlappedComponent :type Primitive%20Component%20Object%20Reference) (OtherActor :type Actor%20Object%20Reference) (OtherComp :type Primitive%20Component%20Object%20Reference) (OtherBodyIndex :type Integer) (bFromSweep :type Boolean) (SweepResult :type Hit%20Result%20Structure%20%28by%20ref%29))
  ;[1 0.7031 0.7031] Not checked | enemy attacking hero and shield
  (bind _asbp_main_hero (Utilities|Casting|CastToBP_MainHero OtherActor)
    (:then
      (Variables|/Script/SuperRPG.BaseCharacter|SetHitPoints _asbp_main_hero (- (Variables|/Script/SuperRPG.BaseCharacter|GetHitPoints _asbp_main_hero) (Variables|Default|GetSpellDamage)))
      (Development|PrintString (Utilities|String|ToString(Float) (- (Variables|/Script/SuperRPG.BaseCharacter|GetHitPoints _asbp_main_hero) (Variables|Default|GetSpellDamage)))))
    (:CastFailed
      (bind _asbp_shield_child (Utilities|Casting|CastToBP_Shield_Child OtherActor))
      (Variables|/Game/Blueprints/Components/Weapon/BP_Shield.BP_Shield_C|SetShieldDefence _asbp_shield_child (- (Variables|/Game/Blueprints/Components/Weapon/BP_Shield.BP_Shield_C|GetShieldDefence _asbp_shield_child) (Variables|Default|GetSpellDamage))))))

(event EventBeginPlay
  ;[1 1 1] Destroy actor in 4 sec
  (Actor|SetLifeSpan 3.0))

(event Collision|EventActorBeginOverlap
  (params (OtherActor :type Actor%20Object%20Reference)))

(event EventTick
  (params (DeltaSeconds :type Float%20%28single-precision%29)))

(fn ConstructionScript)