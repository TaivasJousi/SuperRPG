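; BP_GoldMedium is a gold pickup that adds AddedGold to the main hero's gold count.
; When anything overlaps its SphereCollision, it gets player character 0 as BP_MainHero without checking the overlapping actor.
; It then raises GoldCount, refreshes the gold display through the hero's WBHealthBar widget, destroys itself and prints a debug message.
; An unconnected game mode cast is left unused.
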(event OnComponentBeginOverlap(SphereCollision)
  (params (OverlappedComponent :type Primitive%20Component%20Object%20Reference) (OtherActor :type Actor%20Object%20Reference) (OtherComp :type Primitive%20Component%20Object%20Reference) (OtherBodyIndex :type Integer) (bFromSweep :type Boolean) (SweepResult :type Hit%20Result%20Structure%20%28by%20ref%29))
  ;[1 1 1] Gold Collecting
  (bind _asbp_main_hero (Utilities|Casting|CastToBP_MainHero (Game|GetPlayerCharacter 0)))
  (Variables|/Game/Blueprints/Characters/BP_MainHero.BP_MainHero_C|SetGoldCount _asbp_main_hero (+ (Variables|/Game/Blueprints/Characters/BP_MainHero.BP_MainHero_C|GetGoldCount _asbp_main_hero) (Variables|Default|GetAddedGold)))
  (Default|UpdateGoldCount (Variables|/Game/Blueprints/Characters/BP_MainHero.BP_MainHero_C|GetWB_HealthBar _asbp_main_hero))
  (Actor|DestroyActor)
  (Development|PrintString "Gold found!"))

(fn ConstructionScript
  (|CallParentFunction))