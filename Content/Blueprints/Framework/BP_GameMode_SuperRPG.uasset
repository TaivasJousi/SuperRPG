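; BP_GameMode_SuperRPG is a game mode Blueprint containing an unfinished or disabled player respawn system.
; BeginPlay, Respawning and OnPLAYERDestroyed are empty, so none of that logic executes.
; Disconnected nodes sketch binding to BP_MainHero's destruction, then spawning and possessing a replacement after a delay and calling Respawning.
; Another orphaned node sets the player character's movement mode to Walking.
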(event Custom|OnPLAYERDestroyed
  (params (DestroyedActor :type Actor%20Object%20Reference)))

(event Custom|Respawning)

(event EventBeginPlay)

(fn ConstructionScript)